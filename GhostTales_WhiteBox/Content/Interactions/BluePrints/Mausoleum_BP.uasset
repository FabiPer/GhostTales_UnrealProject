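; Interactable mausoleum actor that shows an interaction prompt and a dialogue widget to the first-person player.
; A prompt box collision shows or hides the prompt Widget component as the FirstPersonCharacter enters or leaves it.
; The Interact event toggles the Mausoleum_Widget on the viewport, creating it for player 0 or removing it if already open.
; Leaving the dialogue box collision also removes and clears the open dialogue.
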(event `self.DialogueBoxCollision.OnComponentEndOverlap`
  (params (OverlappedComponent :type "PrimitiveComponent Object Reference") (OtherActor :type "Actor Object Reference") (OtherComp :type "PrimitiveComponent Object Reference") (OtherBodyIndex :type Integer))
  ;[1 1 1] Removes dialogue after walking away
  (cast `/Game/FirstPersonBP/Blueprints/FirstPersonCharacter` OtherActor)
  (`Widget.RemoveFromParent` (`self.Mausoleum_Widget`))
  (set `self.Mausoleum_Widget` null))

(event `/Game/Interactions/Interact_I.Interact`
  ;[1 1 1] Shows Dialogue
  (`/Engine/EditorBlueprintResources/StandardMacros.IsValid` (`self.Mausoleum_Widget`)
    (:`Is Valid`
      (`Widget.RemoveFromParent` (`self.Mausoleum_Widget`))
      (set `self.Mausoleum_Widget` null))
    (:`Is Not Valid`
      (bind _returnvalue (`|CreateWidget` "/Game/Interactions/Mausoleum_Widget.Mausoleum_Widget_C" (`GameplayStatics.GetPlayerController` 0)))
      (bind _output_get (set `self.Mausoleum_Widget` _returnvalue))
      (`UserWidget.AddToViewport` _output_get 0))))

(event `self.PromptBoxCollision.OnComponentBeginOverlap`
  (params (OverlappedComponent :type "PrimitiveComponent Object Reference") (OtherActor :type "Actor Object Reference") (OtherComp :type "PrimitiveComponent Object Reference") (OtherBodyIndex :type Integer) (bFromSweep :type Boolean) (SweepResult :type "HitResult Structure (by ref)"))
  ;[1 1 1] Shows Prompt
  (cast `/Game/FirstPersonBP/Blueprints/FirstPersonCharacter` OtherActor)
  (`SceneComponent.SetHiddenInGame` (`self.Widget`) false false))

(event `self.PromptBoxCollision.OnComponentEndOverlap`
  (params (OverlappedComponent :type "PrimitiveComponent Object Reference") (OtherActor :type "Actor Object Reference") (OtherComp :type "PrimitiveComponent Object Reference") (OtherBodyIndex :type Integer))
  ;[1 1 1] Hides Prompt
  (cast `/Game/FirstPersonBP/Blueprints/FirstPersonCharacter` OtherActor)
  (`SceneComponent.SetHiddenInGame` (`self.Widget`) true false))

(fn `UserConstructionScript`)