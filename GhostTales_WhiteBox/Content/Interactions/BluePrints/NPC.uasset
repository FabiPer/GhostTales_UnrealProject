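; Interactable NPC that shows a prompt when the player is near and plays data-table dialogue, turning to face the player.
; At BeginPlay it caches the Dialogue__Sheet1 rows matching its NPCID.
; Each Interact advances LineID and displays the line for the current ConversationID in a reused or newly created widget.
; Without exactly one match it closes the widget and resets LineID; leaving the dialogue box also closes it.
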(event `self.DialogueBoxCollision.OnComponentEndOverlap`
  (params (OverlappedComponent :type "PrimitiveComponent Object Reference") (OtherActor :type "Actor Object Reference") (OtherComp :type "PrimitiveComponent Object Reference") (OtherBodyIndex :type Integer))
  ;[1 1 1] Dialogue
  (cast `/Game/FirstPersonBP/Blueprints/FirstPersonCharacter` OtherActor)
  (`Widget.RemoveFromParent` (`self.DialogueWidget`))
  (set `self.DialogueWidget` null))

(event `self.ReceiveBeginPlay`
  ;[1 1 1] Dialogue
  (bind _outrownames (`DataTableFunctionLibrary.GetDataTableRowNames` "/Game/Interactions/Dialogue_-_Sheet1.Dialogue_-_Sheet1"))
  (for _array_element _outrownames
    (bind _returnvalue (`|GetDataTableRow` "/Game/Interactions/Dialogue_-_Sheet1.Dialogue_-_Sheet1" _array_element)
      (:`then`
        (if (== (`.NPC_ID_3_61C1110C42479A58CC8BDFAECE40A45E` (break `/Game/Interactions/DialogueStructure` _returnvalue)) (`self.NPC_ID`))
          (`KismetArrayLibrary.Array_Add` (`self.Dialogue`) _array_element))))))

(event `/Game/Interactions/Interact_I.Interact`
  ;[1 1 1] Turns to look at player
  (`/Engine/EditorBlueprintResources/StandardMacros.IncrementInt` (`self.Line_ID`)
    (:`  `
      (`self.DialogueCreate`)
      (`self.K2_SetActorRotation` (`KismetMathLibrary.MakeRotator` 0.0 0.0 (.yaw (`KismetMathLibrary.FindLookAtRotation` (`self.K2_GetActorLocation`) (`self.K2_GetActorLocation` (`GameplayStatics.GetPlayerCharacter` 0)))))))))

(event `self.PromptBoxCollision.OnComponentBeginOverlap`
  (params (OverlappedComponent :type "PrimitiveComponent Object Reference") (OtherActor :type "Actor Object Reference") (OtherComp :type "PrimitiveComponent Object Reference") (OtherBodyIndex :type Integer) (bFromSweep :type Boolean) (SweepResult :type "HitResult Structure (by ref)"))
  ;[1 1 1] Shows Prompt
  (cast `/Game/FirstPersonBP/Blueprints/FirstPersonCharacter` OtherActor)
  (`SceneComponent.SetHiddenInGame` (`self.Prompt Widget`) false false))

(event `self.PromptBoxCollision.OnComponentEndOverlap`
  (params (OverlappedComponent :type "PrimitiveComponent Object Reference") (OtherActor :type "Actor Object Reference") (OtherComp :type "PrimitiveComponent Object Reference") (OtherBodyIndex :type Integer))
  ;[1 1 1] Hides Prompt
  (cast `/Game/FirstPersonBP/Blueprints/FirstPersonCharacter` OtherActor)
  (`SceneComponent.SetHiddenInGame` (`self.Prompt Widget`) true false))

(fn `DialogueCreate`
  (`/Engine/EditorBlueprintResources/StandardMacros.IsValid` (`self.DialogueWidget`)
    (:`Is Valid`
      (bind _returnedline (`self.DialogueGetLine`))
      (set `/Game/Interactions/Widgets/DialogueWidget.DialogueText` _returnedline (`self.DialogueWidget`)))
    (:`Is Not Valid`
      (bind _returnvalue (`|CreateWidget` "/Game/Interactions/Widgets/DialogueWidget.DialogueWidget_C" (`GameplayStatics.GetPlayerController` 0)))
      (bind _output_get (set `self.DialogueWidget` _returnvalue))
      (`UserWidget.AddToViewport` _output_get 0)
      (bind _returnedline_2 (`self.DialogueGetLine`))
      (set `/Game/Interactions/Widgets/DialogueWidget.DialogueText` _returnedline_2 (`self.DialogueWidget`)))))

(fn `DialogueGetLine`
  (returns (returnedLine :type Text))
  (locals (ReturnedLines :type "Array of Text"))
  (for _array_element (`self.Dialogue`)
    (bind _returnvalue (`|GetDataTableRow` "/Game/Interactions/Dialogue_-_Sheet1.Dialogue_-_Sheet1" _array_element)
      (:`then`
        (bind (_npc_id _conversation_id _line_id _dialogue) (break `/Game/Interactions/DialogueStructure` _returnvalue))
        (if (and (== _conversation_id (`self.Conversation_ID`)) (== _line_id (`self.Line_ID`)))
          (`KismetArrayLibrary.Array_Add` (`local.ReturnedLines`) _dialogue)))))
  (if (== (`KismetArrayLibrary.Array_Length` (`local.ReturnedLines`)) 1)
    (return (`|GetArrayItem` (`local.ReturnedLines`)))
    (else
      (`Widget.RemoveFromParent` (`self.DialogueWidget`))
      (set `self.DialogueWidget` null)
      (set `self.Line_ID` 0))))

(fn `UserConstructionScript`)